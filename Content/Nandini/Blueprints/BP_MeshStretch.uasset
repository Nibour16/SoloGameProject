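; BP_MeshStretch is a construction-script tool that repeats a chosen mesh along a spline as deformed spline mesh segments with configurable collision.
; It places segments at fixed section-length intervals, clamping tangents to that length.
; UseFullLegthMesh keeps only whole sections, otherwise one more segment covers the remainder.
; With AllowScaling on, the script only derives section length from actor X scale and builds no meshes.
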(fn `Get End Pos/Tangent`
  (params (Index :type Integer))
  (returns (Position :type "Vector Structure") (Tangent :type "Vector Structure"))
  (bind _spline (`self.Spline`))
  (bind _returnvalue (* (+ Index 1) (`self.ScetionLength`)))
  (return (`SplineComponent.GetLocationAtDistanceAlongSpline` _spline _returnvalue "Local") (`KismetMathLibrary.ClampVectorSize` (`SplineComponent.GetTangentAtDistanceAlongSpline` _spline _returnvalue "Local") 0.0 (`self.ScetionLength`))))

(fn `Get Start Pos/Tangent`
  (params (Index :type Integer))
  (returns (Position :type "Vector Structure") (Tangent :type "Vector Structure"))
  (bind _spline (`self.Spline`))
  (bind _returnvalue (* Index (`self.ScetionLength`)))
  (return (`SplineComponent.GetLocationAtDistanceAlongSpline` _spline _returnvalue "Local") (`KismetMathLibrary.ClampVectorSize` (`SplineComponent.GetTangentAtDistanceAlongSpline` _spline _returnvalue "Local") 0.0 (`self.ScetionLength`))))

(fn `UserConstructionScript`
  (bind _returnvalue_x (`KismetMathLibrary.BreakVector` (`self.GetActorScale3D`)))
  (if (`self.AllowScaling?`)
    (set `self.ScetionLength` (* _returnvalue_x 100.0))
    (elif (`self.UseFullLegthMesh?`)
      (for _index (range (`KismetMathLibrary.FTrunc` (/ (`SplineComponent.GetSplineLength` (`self.Spline`)) (`self.ScetionLength`))))
        (set `self.LoopIndex` _index)
        (bind _returnvalue (`AddComponent|NODE_AddSplineMeshComponent-0` :!label _label))
        (`StaticMeshComponent.SetStaticMesh` _returnvalue (`self.Mesh`))
        (`SplineMeshComponent.SetForwardAxis` _returnvalue "X" true)
        (bind (_position _tangent) (`self.Get Start Pos/Tangent` (`self.LoopIndex`)))
        (bind (_position_2 _tangent_2) (`self.Get End Pos/Tangent` (`self.LoopIndex`)))
        (`SplineMeshComponent.SetStartAndEnd` _returnvalue _position _tangent _position_2 _tangent_2 true)
        (`PrimitiveComponent.SetCollisionEnabled` _returnvalue (`self.Collision`)))
      (else
        (for _index_2 (range (+ (`KismetMathLibrary.FTrunc` (/ (`SplineComponent.GetSplineLength` (`self.Spline`)) (`self.ScetionLength`))) 1))
          (set `self.LoopIndex` _index_2)
          (goto _label))))))