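; BP_WallButton is a wall switch that stays on while at least one BP_Arrow overlaps its Button component.
; Overlap begin and end events on Button raise and lower a count of triggering arrows, ignoring other actors.
; Tick calls SetSwitch every frame, passing true while that count is above zero and false otherwise.
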(event `self.ReceiveTick`
  (params (DeltaSeconds :type "Float (single-precision)"))
  ; Update if one of player's arrows is colliding with the button
  (if (> (`self.#OfTriggeringArrows`) 0)
    (`self.SetSwitch` true)
    (else
      (`self.SetSwitch` false))))

(event `self.Button.OnComponentBeginOverlap`
  (params (OverlappedComponent :type "PrimitiveComponent Object Reference") (OtherActor :type "Actor Object Reference") (OtherComp :type "PrimitiveComponent Object Reference") (OtherBodyIndex :type Integer) (bFromSweep :type Boolean) (SweepResult :type "HitResult Structure (by ref)"))
  ; Player projectiles that triggers it will be counted as trigger arrows
  (cast `/Game/RobinProto/Blueprints/Characters/Projectiles/BP_Arrow` OtherActor)
  (set `self.#OfTriggeringArrows` (+ (`self.#OfTriggeringArrows`) 1)))

(event `self.Button.OnComponentEndOverlap`
  (params (OverlappedComponent :type "PrimitiveComponent Object Reference") (OtherActor :type "Actor Object Reference") (OtherComp :type "PrimitiveComponent Object Reference") (OtherBodyIndex :type Integer))
  ; Subtract one from trigger arrow number when an arrow is removed
  (cast `/Game/RobinProto/Blueprints/Characters/Projectiles/BP_Arrow` OtherActor)
  (set `self.#OfTriggeringArrows` (- (`self.#OfTriggeringArrows`) 1)))

(fn `UserConstructionScript`
  (`parent.UserConstructionScript`))