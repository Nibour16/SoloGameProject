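; BP_BaseButton is a switch button that stays on while at least one triggerer, noted as the player's arrows, is on it.
; An update event waits a tick, then adds a change to the triggerer count.
; Tick sets the inherited switch state on or off from whether that count is above zero.
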(event `self.ReceiveTick`
  (params (DeltaSeconds :type "Float (single-precision)"))
  ; Update if one of player's arrows is colliding with the button
  (if (> (`self.#OfTriggerer`) 0)
    (`self.SetSwitch` true)
    (else
      (`self.SetSwitch` false))))

(event `Update#OfTriggerer`
  (params (NumberChange :type Integer))
  ; Set # Of Triggerer
  (`KismetSystemLibrary.DelayUntilNextTick`)
  (set `self.#OfTriggerer` (+ (`self.#OfTriggerer`) NumberChange)))

(fn `UserConstructionScript`
  (`parent.UserConstructionScript`))