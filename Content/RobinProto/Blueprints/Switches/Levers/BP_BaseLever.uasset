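; BP_BaseLever is a base lever switch that the player toggles through interaction.
; Each Interact by a BP_Player sets IsInteracting and alternates playing or reversing a timeline that rotates the stick's roll between ClosedRotation and OpenedRotation.
; When the animation finishes, it clears IsInteracting and calls SetSwitch with the FlipFlop state.
; The construction script places the stick at its closed rotation.
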(event `/Game/RobinProto/Blueprints/Utilities/BI_Interactable.Interact`
  (params (Interactor :type "Actor Object Reference"))
  ; Interaction with Lever
  (bind _asbp_player (cast `/Game/RobinProto/Blueprints/Characters/Player/Blueprints/BP_Player` Interactor))
  (set `/Game/RobinProto/Blueprints/Characters/Player/Blueprints/BP_Player.IsInteracting` true _asbp_player)
  (bind _isa (`/Engine/EditorBlueprintResources/StandardMacros.FlipFlop`)
    (:`A`
      (bind (_direction _levertrackalpha) (`Timeline|Timeline_Lever` :!label _label)
        (:`Update`
          (`SceneComponent.K2_SetRelativeRotation` (`self.SM_LeverStick`) (`KismetMathLibrary.RLerp` (`KismetMathLibrary.MakeRotator` (`self.ClosedRotation`)) (`KismetMathLibrary.MakeRotator` (`self.OpenedRotation`)) _levertrackalpha) false false))
        (:`Finished`
          ;; Finish Animation
          (set `/Game/RobinProto/Blueprints/Characters/Player/Blueprints/BP_Player.IsInteracting` false _asbp_player)
          (`self.SetSwitch` _isa))))
    (:`B`
      (goto _label :!via `Reverse`))))

(fn `UserConstructionScript`
  ; Initialize Lever
  (`SceneComponent.K2_SetRelativeRotation` (`self.SM_LeverStick`) (`KismetMathLibrary.MakeRotator` (`self.ClosedRotation`)) false false))