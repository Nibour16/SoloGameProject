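; BP_SwitchDoor is a door that moves vertically between a closed and an open position based on its Switch state.
; On BeginPlay, ZPosInitializer processes InitialPos and FinalPos against the Door reference and stores the results.
; Every Tick, SwitchDoorUpDown receives the door, the Switch flag and both positions, using InitialPos as down and FinalPos as up.
; Both helpers are defined outside this graph, and the construction script only calls its parent.
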(event `self.ReceiveBeginPlay`
  ; Initialization
  (bind _newpos (`self.ZPosInitializer` (`self.Door`) (`self.InitialPos`)))
  (set `self.InitialPos` _newpos)
  (bind _newpos_2 (`self.ZPosInitializer` (`self.Door`) (`self.FinalPos`)))
  (set `self.FinalPos` _newpos_2))

(event `self.ReceiveTick`
  (params (DeltaSeconds :type "Float (single-precision)"))
  ; Update Door Open/Close
  (`self.Switch_Door(Up/Down)` (`self.Door`) (`self.Switch`) (`self.InitialPos`) (`self.FinalPos`)))

(fn `UserConstructionScript`
  (`parent.UserConstructionScript`))