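; Base switch door Blueprint that slides a supplied door component vertically between down and up Z positions.
; The Switch_Door event drives the OpenCloseDoor timeline, playing it to open and reversing it to close, with updates lerping relative location.
; A first-time flag suppresses movement until the first open finishes, so an initial close does nothing.
; ZPosInitializer computes a target Z by adding an offset to the door's relative Z.
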(event `Switch_Door(Up/Down)`
  (params (DoorRef :type "SceneComponent Object Reference") (IsOpen :type Boolean) (DownVectorZ :type "Float (double-precision)") (UpVectorZ :type "Float (double-precision)"))
  ; Check If it is opened/closed. If it is first time to switch will not move the door
  (if (`self.IsFirstTimeToSwitch`)
    (if IsOpen
      ; Make up/down movement for the door. Once it finishes will set the first time boolean to false
      (bind (_direction _updownmovementtrackalpha) (`Timeline|Open/Close Door` :!label _label)
        (:`Update`
          (`SceneComponent.K2_SetRelativeLocation` DoorRef (`KismetMathLibrary.VLerp` (`KismetMathLibrary.MakeVector` 0.0 0.0 DownVectorZ) (`KismetMathLibrary.MakeVector` 0.0 0.0 UpVectorZ) _updownmovementtrackalpha) false false))
        (:`Finished`
          (set `self.IsFirstTimeToSwitch` false))))
    (elif IsOpen
      (goto _label)
      (else
        (goto _label :!via `Reverse`)))))

(fn `UserConstructionScript`)

(fn `ZPosInitializer`
  (params (DoorRef :type "SceneComponent Object Reference") (InputPos :type "Float (double-precision)"))
  (returns (NewPos :type "Float (double-precision)"))
  (bind (_relativelocation_x _relativelocation_y _relativelocation_z) (`KismetMathLibrary.BreakVector` (`SceneComponent.RelativeLocation` DoorRef)))
  (return (+ _relativelocation_z InputPos)))