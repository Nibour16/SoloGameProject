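; Game instance for the solo game that holds the BP_SaveGame object and handles loading, saving and checkpoint cleanup.
; Init loads the BP_Checkpoint slot, with CheckSaveFile creating a fresh save object if none exists, and Shutdown deletes that slot.
; Load and save support async or blocking calls, though only async loading fires OnGameLoaded.
; SavePlayer writes player data then saves, while helpers return the save object or actor transforms by class.
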(event `self.ReceiveInit`
  ; Initialization
  (bind _returnvalue (`GameplayStatics.GetActorOfClass` "/Game/Robin/Blueprint/DataSave/BP_Checkpoint.BP_Checkpoint_C"))
  (`self.LoadData` false (`/Game/Robin/Blueprint/DataSave/BP_Checkpoint.Slot Name` _returnvalue)))

(event `/Game/Robin/Blueprint/Utilities/BI_SaveGame.LoadData`
  (params (Async :type Boolean) (SlotName :type String))
  ; Load Data Event
  (`self.CheckSaveFile` SlotName
    (:`then`
      ;;[1 1 1] Check Async
      (if Async
        ;;[1 1 1] Aysnc Load Game
        (bind _savegame (`AsyncActionHandleSaveGame.AsyncLoadGameFromSlot` SlotName)
          (:`Completed`
            (bind _asbp_save_game (cast `/Game/Robin/Blueprint/DataSave/BP_SaveGame` _savegame))
            (set `self.SaveGameDataRef` _asbp_save_game)
            (`self.OnGameLoaded`)))
        (else
          ;;[1 1 1] Load Game
          (bind _returnvalue (`GameplayStatics.LoadGameFromSlot` SlotName))
          (bind _asbp_save_game_2 (cast `/Game/Robin/Blueprint/DataSave/BP_SaveGame` _returnvalue))
          (set `self.SaveGameDataRef` _asbp_save_game_2))))))

(event `/Game/Robin/Blueprint/Utilities/BI_SaveGame.SaveData`
  (params (Async :type Boolean) (SlotName :type String))
  ; Save Data Event
  ;;[1 1 1 1 14] Check Async
  (if Async
    (`AsyncActionHandleSaveGame.AsyncSaveGameToSlot` (`self.SaveGameDataRef`) SlotName)
    (else
      (`GameplayStatics.SaveGameToSlot` (`self.SaveGameDataRef`) SlotName))))

(event `self.ReceiveShutdown`
  ; Delete Checkpoint if the game has been shutdown immediately
  (bind _returnvalue (`GameplayStatics.GetActorOfClass` "/Game/Robin/Blueprint/DataSave/BP_Checkpoint.BP_Checkpoint_C"))
  (`GameplayStatics.DeleteGameInSlot` (`/Game/Robin/Blueprint/DataSave/BP_Checkpoint.Slot Name` _returnvalue)))

(event `/Game/Robin/Blueprint/Utilities/BI_SaveGame.SavePlayer`
  (params (Async :type Boolean) (PlayerData :type "/Game/Robin/Blueprint/DataSave/Structures/S_Player Structure") (SlotName :type String))
  ; Save Player
  (set `/Game/Robin/Blueprint/DataSave/BP_SaveGame.PlayerData` PlayerData (`self.SaveGameDataRef`))
  (`self.SaveData` Async SlotName))

(fn `GetData`
  (returns (SaveData :type "/Game/Robin/Blueprint/DataSave/BP_SaveGame Object Reference"))
  (return (`self.SaveGameDataRef`)))

(fn `SaveTransform`
  (params (ActorToSave :type "Actor Class Reference"))
  (returns (OutputTransform :type "Array of Transform Structure"))
  (locals (Array :type "Array of Transform Structure"))
  (`KismetArrayLibrary.Array_Clear` (`local.Array`))
  (bind _outactors (`GameplayStatics.GetAllActorsOfClass` ActorToSave))
  (for _array_element _outactors
    ;[1 1 1] Add Data
    (`KismetArrayLibrary.Array_Add` (`local.Array`) (`Actor.GetTransform` _array_element)))
  (return (`local.Array`)))