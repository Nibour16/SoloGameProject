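; Player bow skeletal mesh component that handles shooting arrows and adds its Enhanced Input mapping context through the game mode on BeginPlay.
; Shoot input checks ammo and busy state, adjusts first-person mesh height, then starts montages on player, bow and arrow meshes together.
; An animation-driven Shoot! event decrements ammo, spawns BP_Arrow with sound and restores mesh height.
; A second input toggles the arrow box display flag with a HUD popup.
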(event EventBeginPlay
  ;[0.15 0.15 0.15 0.5] Player Ref Setup
  (bind _asbp_player (Utilities|Casting|CastToBP_Player (Components|GetOwner)))
  (Variables|Default|SetPlayerRef _asbp_player)
  ;[0.05 0.05 0.05] With enhanced input we can add a new mapping context that configures the shoot action and enable the input. This could also be removed when the player drops the weapon. In this way you could even make updates to the base game introducing new input layouts without a monolitic long Default Input.ini
  (bind _asbp_solo_game_mode (Utilities|Casting|CastToBP_SoloGameMode (Game|GetGameMode)))
  (Default|MappingContextSetup _asbp_solo_game_mode (Pawn|GetController (Variables|Default|GetPlayerRef)) "/Game/RobinProto/Blueprints/Characters/Player/Input/IMC_Gun.IMC_Gun"))

(event Input|EnhancedActionEvents|EnhancedInputActionIA_Shoot
  (params (ActionValue :type Boolean) (ElapsedSeconds :type Float%20%28double-precision%29) (TriggeredSeconds :type Float%20%28double-precision%29) (InputAction :type Input%20Action%20Object%20Reference :default "/Game/RobinProto/Blueprints/Characters/Player/Input/Actions/IA_Shoot.IA_Shoot"))
  (bind _playerref (Variables|Default|GetPlayerRef))
  ;[0.1031 0.1031 0.1031 0.502] Check Ammoes
  (if (> (Variables|/Game/RobinProto/Blueprints/Characters/Player/Blueprints/BP_Player.BP_Player_C|GetCurrentAmmoes (Variables|Default|GetPlayerRef)) 0)
    ;[0.15 0.15 0.15 0.5] Handle Shooting
    (if (Variables|Default|GetIsNotShooting)
      (Variables|Default|SetIsNotShooting false)
      (Utilities|SetMeshHeight (Variables|/Game/RobinProto/Blueprints/Characters/Player/Blueprints/BP_BasePlayer.BP_BasePlayer_C|GetFirstPersonMesh _playerref) (Variables|Default|GetZPosWhileAiming))
      ;;[0.3515 0.3515 0.3515 0.502] Attack Montage Play
      (Utilities|PlayAttackMontage (Variables|/Game/RobinProto/Blueprints/Characters/Player/Blueprints/BP_BasePlayer.BP_BasePlayer_C|GetFirstPersonMesh _playerref) "/Game/Robin/Art/Player/AM_PlayerAttack.AM_PlayerAttack"
        (:then
          (Utilities|PlayAttackMontage self "/Game/Smooztime/Player/Bow_Attack_Montage.Bow_Attack_Montage"
            (:then
              (Utilities|PlayAttackMontage (Variables|/Game/RobinProto/Blueprints/Characters/Player/Blueprints/BP_Player.BP_Player_C|GetArrowSKRef _playerref) "/Game/Robin/Art/Player/AM_Arrow.AM_Arrow"
                (:On%20Completed
                  _)
                (:On%20Interrupted
                  (Utilities|SetMeshHeight (Variables|/Game/RobinProto/Blueprints/Characters/Player/Blueprints/BP_BasePlayer.BP_BasePlayer_C|GetFirstPersonMesh (Variables|Default|GetPlayerRef)) (Variables|Default|GetZPosInitial))))
              (Variables|Default|SetIsNotShooting true)))))
      (else
        (Development|PrintString "Delaying")))
    (else
      (Development|PrintString "Out of Arrows!"))))

(event Input|EnhancedActionEvents|EnhancedInputActionIA_ShowBox
  (params (ActionValue :type Boolean) (ElapsedSeconds :type Float%20%28double-precision%29) (TriggeredSeconds :type Float%20%28double-precision%29) (InputAction :type Input%20Action%20Object%20Reference :default "/Game/RobinProto/Blueprints/Characters/Player/Input/Actions/IA_ShowBox.IA_ShowBox"))
  ;[0.15 0.15 0.15 0.5] Show Arrow Steppable Box
  (:Started
    (Utilities|FlowControl|FlipFlop
      (:A
        (Variables|Default|SetIsDisplayedArrowBox false))
      (:B
        (Variables|Default|SetIsDisplayedArrowBox true)))
    (bind _foundwidgets (Widget|GetAllWidgetsOfClass (Variables|/Game/RobinProto/Blueprints/Characters/Player/Blueprints/BP_Player.BP_Player_C|GetPlayerHUDClass (Variables|Default|GetPlayerRef)) true))
    (Default|PopupSwitchInfo (Utilities|Array|Get(acopy) _foundwidgets) (Variables|/Game/RobinProto/Blueprints/UI/HUD/WBP_PlayerHUD.WBP_PlayerHUD_C|GetArrowBoxDisplayInfo (Utilities|Array|Get(acopy) _foundwidgets)) (Variables|/Game/RobinProto/Blueprints/UI/HUD/WBP_PlayerHUD.WBP_PlayerHUD_C|GetArrowBoxHiddenInfo (Utilities|Array|Get(acopy) _foundwidgets)) 3.0 (Variables|Default|GetIsDisplayedArrowBox))))

(event Custom|Shoot!
  (bind _returnvalue (|GetShootTransform))
  (bind _playerref (Variables|Default|GetPlayerRef))
  ;[0.05 0.05 0.05] Projectile Spawn Logic
  (bind _result (Math|Integer|DecrementInt (Variables|/Game/RobinProto/Blueprints/Characters/Player/Blueprints/BP_Player.BP_Player_C|GetCurrentAmmoes _playerref))
    (:%20%20
      (Variables|/Game/RobinProto/Blueprints/Characters/Player/Blueprints/BP_Player.BP_Player_C|SetCurrentAmmoes _playerref _result)
      (Game|SpawnActorfromClass "/Game/RobinProto/Blueprints/Characters/Projectiles/BP_Arrow.BP_Arrow_C" (Math|Transform|MakeTransform (.location _returnvalue) (.rotation _returnvalue) (.scale _returnvalue)) "AdjustIfPossibleButAlwaysSpawn" "OverrideRootScale" 0 0)
      (Audio|PlaySoundatLocation (Variables|Default|GetShootingSound) (.location _returnvalue) "0, 0, 0" 1.0 1.0 0.0 0 0 0 0)
      ;[0.15 0.15 0.15 0.5] Reset Mesh Height
      (Utilities|SetMeshHeight (Variables|/Game/RobinProto/Blueprints/Characters/Player/Blueprints/BP_BasePlayer.BP_BasePlayer_C|GetFirstPersonMesh (Variables|Default|GetPlayerRef)) (Variables|Default|GetZPosInitial)))))