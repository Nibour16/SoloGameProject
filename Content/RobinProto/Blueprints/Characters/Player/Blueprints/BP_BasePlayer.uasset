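; BP_BasePlayer is a base player Blueprint that sets up player input and popup menus.
; On a controller change it waits one tick, then asks the game mode to apply the IMC_Player mapping context to the new controller.
; On BeginPlay it runs the parent logic, then creates a hidden WBP_BaseWidget in the viewport and has it build submenus from the PopupMenusClasses list.
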(event `self.ReceiveControllerChanged`
  (params (OldController :type "Controller Object Reference") (NewController :type "Controller Object Reference"))
  ; Input Mapping Context
  (`KismetSystemLibrary.DelayUntilNextTick`)
  (`/Game/RobinProto/Blueprints/BP_SoloGameMode.MappingContextSetup` (`self.GameModeRef`) NewController "/Game/RobinProto/Blueprints/Characters/Player/Input/IMC_Player.IMC_Player"))

(event `self.ReceiveBeginPlay`
  ; Initial Blueprint
  (`parent.ReceiveBeginPlay`)
  (`self.MenuSetup` (`self.PopupMenusClasses`)))

(event `MenuSetup`
  (params (SubMenuArray :type "Array of /Game/RobinProto/Blueprints/UI/WBP_BaseWidget Class Reference (by ref)"))
  ; Menu Setup
  (bind _output (`self.GetBaseWidgetClass`))
  (`/Game/RobinProto/Blueprints/UI/WBP_BaseWidget.CreateSubMenus` _output SubMenuArray))

(fn `GetBaseWidgetClass`
  (returns (Output :type "/Game/RobinProto/Blueprints/UI/WBP_BaseWidget Object Reference"))
  (bind _returnvalue (`|CreateWidget` "/Game/RobinProto/Blueprints/UI/WBP_BaseWidget.WBP_BaseWidget_C"))
  (`UserWidget.AddToViewport` _returnvalue 0)
  (`Widget.SetVisibility` _returnvalue "Hidden")
  (return _returnvalue))

(fn `UserConstructionScript`
  (`parent.UserConstructionScript`))