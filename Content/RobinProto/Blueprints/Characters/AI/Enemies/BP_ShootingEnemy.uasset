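; BP_ShootingEnemy is an AI enemy that carries a gun and fires projectiles.
; The construction script attaches the gun to the mesh's right-hand socket.
; AI perception updates pass to PlayerDetection with the sight sense for spotting the player.
; The ShootProjectile event spawns the configured projectile class at the ShootingPos component's location plus an offset, using that component's rotation.
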(event `ShootProjectile`
  (bind _shootingpos (`self.ShootingPos`))
  ; Shoot a projectile
  (`|SpawnActorFromClass` (`self.ProjectileClass`) (`KismetMathLibrary.MakeTransform` (+ (`SceneComponent.K2_GetComponentLocation` _shootingpos) (`self.ProjectileOffset`)) (`SceneComponent.K2_GetComponentRotation` _shootingpos)) "Undefined" "MultiplyWithRoot" null null))

(event `self.AIPerception.OnTargetPerceptionUpdated`
  (params (Actor :type "Actor Object Reference") (Stimulus :type "AIStimulus Structure"))
  ; Seeing Player
  (`self.PlayerDetection` Actor Stimulus "/Script/AIModule.AISense_Sight"))

(fn `UserConstructionScript`
  (`SceneComponent.K2_AttachToComponent` (`self.Gun`) (`self.Mesh`) "hand_r_gunSocket" "KeepRelative" "KeepRelative" "KeepRelative" true))