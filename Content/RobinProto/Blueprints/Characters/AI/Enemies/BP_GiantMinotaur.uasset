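; BP_GiantMinotaur is a giant minotaur enemy Blueprint that defines how the creature reacts to taking damage.
; Its AnyDamage event passes damage to GetDamaged only while CanDamageChar is true.
; If the actor is still valid afterward, it calls CharInvincible on itself and prints a "Moo!!!!" message.
; BeginPlay, overlap and the construction script add no logic of their own.
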(event `self.ReceiveAnyDamage`
  (params (Damage :type "Float (single-precision)") (DamageType :type "DamageType Object Reference") (InstigatedBy :type "Controller Object Reference") (DamageCauser :type "Actor Object Reference"))
  (if (`self.CanDamageChar`)
    (`self.GetDamaged` Damage)
    (`/Engine/EditorBlueprintResources/StandardMacros.IsValid` self
      (:`Is Valid`
        (`self.CharInvincible` self)
        (`KismetSystemLibrary.PrintString` "Moo!!!!")))))

(fn `UserConstructionScript`
  (`parent.UserConstructionScript`))