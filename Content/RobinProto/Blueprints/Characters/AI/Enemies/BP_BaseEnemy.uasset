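; Base enemy Blueprint that damages the player on contact and destroys itself when it dies.
; An AttackBox overlap starts a short-delay loop that retries hits until the player leaves, applying damage only while the player's CanDamageChar is true.
; Damage and knockback forces route through BP_SoloGameMode's DamageCharacter.
; PlayerDetection forwards sensed stimuli to BP_AIController's HandleSensing, with the player character as target.
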(event `self.ReceiveBeginPlay`
  ; Parent Begin Play
  (`parent.ReceiveBeginPlay`))

(event `/Game/RobinProto/Blueprints/Utilities/BI_Character.Die`
  ; When died
  (`self.K2_DestroyActor`))

(event `self.AttackBox.OnComponentBeginOverlap`
  (params (OverlappedComponent :type "PrimitiveComponent Object Reference") (OtherActor :type "Actor Object Reference") (OtherComp :type "PrimitiveComponent Object Reference") (OtherBodyIndex :type Integer) (bFromSweep :type Boolean) (SweepResult :type "HitResult Structure (by ref)"))
  ; When Catches Player
  (set `self.IsHitting` true)
  (if (`self.IsHitting`) :!label _label
    (`KismetSystemLibrary.Delay` 0.01)
    (`self.HitPlayer` OtherActor)
    (goto _label)))

(event `self.AttackBox.OnComponentEndOverlap`
  (params (OverlappedComponent :type "PrimitiveComponent Object Reference") (OtherActor :type "Actor Object Reference") (OtherComp :type "PrimitiveComponent Object Reference") (OtherBodyIndex :type Integer))
  ; Player Escapes from collision
  (cast `/Game/RobinProto/Blueprints/Characters/Player/Blueprints/BP_Player` OtherActor)
  (set `self.IsHitting` false))

(event `HitPlayer`
  (params (PlayerActor :type "Actor Object Reference"))
  ; Hit Player
  (bind _asbp_player (cast `/Game/RobinProto/Blueprints/Characters/Player/Blueprints/BP_Player` PlayerActor))
  (if (`/Game/RobinProto/Blueprints/Characters/BP_BaseCharacter.CanDamageChar` _asbp_player)
    (`self.DamagePlayer` _asbp_player self (`self.HitDamage`))))

(event `PlayerDetection`
  (params (Actor :type "Actor Object Reference") (Stimulus :type "AIStimulus Structure") (SenseType :type "Object Class Reference"))
  ; Sense Player (Cache the AI controller as a variable)
  (bind _asbp_aicontroller (cast `/Game/RobinProto/Blueprints/Characters/AI/BP_AIController` (`AIBlueprintHelperLibrary.GetAIController` self)))
  (`/Game/RobinProto/Blueprints/Characters/AI/BP_AIController.HandleSensing` _asbp_aicontroller Actor Stimulus (`GameplayStatics.GetPlayerCharacter` 0) SenseType))

(fn `DamagePlayer`
  (params (DamagedPlayer :type "/Game/RobinProto/Blueprints/Characters/Player/Blueprints/BP_Player Object Reference") (DamageCauser :type "Actor Object Reference") (BaseDamage :type "Float (single-precision)"))
  ; Enemy Damage Player
  (bind _asbp_solo_game_mode (cast `/Game/RobinProto/Blueprints/BP_SoloGameMode` (`GameplayStatics.GetGameMode`)))
  (`/Game/RobinProto/Blueprints/BP_SoloGameMode.DamageCharacter` _asbp_solo_game_mode DamagedPlayer BaseDamage null DamageCauser null (`self.KnockbackMainForce`) (`self.KnockbackForceUp`) true))

(fn `UserConstructionScript`
  (`parent.UserConstructionScript`))