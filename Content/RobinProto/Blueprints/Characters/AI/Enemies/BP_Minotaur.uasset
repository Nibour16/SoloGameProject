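; BP_Minotaur is an enemy character that carries an axe attached to the right-hand weapon socket of its mesh at construction.
; It caches the player pawn on BeginPlay.
; StartDamaging starts a fast looping timer that damages the player by its Attack value while the HitBox overlaps them, and FinishDamaging clears it.
; Hits are not deduplicated, so damage can repeat on every timer tick unless handled elsewhere.
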(event `self.ReceiveBeginPlay`
  ; Initialization
  (`parent.ReceiveBeginPlay`)
  (bind _asbp_player (cast `/Game/RobinProto/Blueprints/Characters/Player/Blueprints/BP_Player` (`GameplayStatics.GetPlayerCharacter` 0)))
  (set `self.PlayerRef` _asbp_player))

(event `StartDamaging`
  ; Start Damage Timer Event
  (bind _returnvalue (`KismetSystemLibrary.K2_SetTimerDelegate` (delegate `OnDamage`) 0.01 true true))
  (set `self.DamageTraceLoop` _returnvalue))

(event `OnDamage`
  (bind _playerref (`self.PlayerRef`))
  ; Deal Damage
  (if (`PrimitiveComponent.IsOverlappingActor` (`self.HitBox`) _playerref)
    (`self.DamagePlayer` _playerref self (`self.Attack`))))

(event `FinishDamaging`
  ; Finish Damage
  (`KismetSystemLibrary.K2_ClearAndInvalidateTimerHandle` (`self.DamageTraceLoop`)))

(fn `UserConstructionScript`
  (`SceneComponent.K2_AttachToComponent` (`self.SM_MinotaurAxe`) (`self.Mesh`) "hand_r_weapon_socket" "KeepRelative" "KeepRelative" "KeepRelative" true)
  (`parent.UserConstructionScript`))