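; BP_EnemyProjectile is a projectile fired by enemies that damages the player on hit.
; On hit with BP_Player, it resolves the firing character from its damage-causer reference, casts it to BP_BaseEnemy, calls DamagePlayer with that character's Attack value, then destroys itself.
; When the projectile movement stops, it waits a set lifetime delay before destroying itself.
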(event `self.ReceiveHit`
  (params (MyComp :type "PrimitiveComponent Object Reference") (Other :type "Actor Object Reference") (OtherComp :type "PrimitiveComponent Object Reference") (bSelfMoved :type Boolean) (HitLocation :type "Vector Structure") (HitNormal :type "Vector Structure") (NormalImpulse :type "Vector Structure") (Hit :type "HitResult Structure (by ref)"))
  ; Hit player
  (bind _asbp_player (cast `/Game/RobinProto/Blueprints/Characters/Player/Blueprints/BP_Player` Other))
  (bind _findref (`self.GetCharRef` (`self.DamCauserRef`)))
  (bind _asbp_base_enemy (cast `/Game/RobinProto/Blueprints/Characters/AI/Enemies/BP_BaseEnemy` _findref))
  (`/Game/RobinProto/Blueprints/Characters/AI/Enemies/BP_BaseEnemy.DamagePlayer` _asbp_base_enemy _asbp_player self (`/Game/RobinProto/Blueprints/Characters/BP_BaseCharacter.Attack` _findref))
  (`self.K2_DestroyActor`))

(event `self.ProjectileMovement.OnProjectileStop`
  (params (ImpactResult :type "HitResult Structure (by ref)"))
  ; Finish Simulation
  (`KismetSystemLibrary.Delay` (`self.ExistingTime`))
  (`self.K2_DestroyActor`))

(fn `UserConstructionScript`
  (`parent.UserConstructionScript`))