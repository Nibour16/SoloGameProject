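; BP_Arrow is a player-collectible arrow projectile that damages enemies and carries a steppable box.
; A hit on an enemy applies the shooter's Attack once, then enables bounce and gravity; other hits disable both.
; Stopping disarms it, and interacting returns one arrow to BP_Player and destroys the actor.
; Tick syncs the box's visibility to the player's gun component, while collisions play an impact sound.
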(event `/Game/RobinProto/Blueprints/Utilities/BI_Interactable.Interact`
  (params (Interactor :type "Actor Object Reference"))
  ; Interact this actor to restore the arrow
  (bind _asbp_player (cast `/Game/RobinProto/Blueprints/Characters/Player/Blueprints/BP_Player` Interactor))
  (`/Game/RobinProto/Blueprints/Characters/Player/Blueprints/BP_Player.CollectArrow` _asbp_player 1)
  (`self.K2_DestroyActor`))

(event `self.ReceiveTick`
  (params (DeltaSeconds :type "Float (single-precision)"))
  ; Show Steppable Box
  (bind _asbp_player (cast `/Game/RobinProto/Blueprints/Characters/Player/Blueprints/BP_Player` (`GameplayStatics.GetPlayerCharacter` 0)))
  (`SceneComponent.SetHiddenInGame` (`self.SteppableBox`) (not (`/Game/RobinProto/Blueprints/Characters/Player/Blueprints/BP_Gun_Component.IsDisplayedArrowBox` (`/Game/RobinProto/Blueprints/Characters/Player/Blueprints/BP_Player.BP_Gun_Component` _asbp_player))) false))

(event `self.ProjectileMovement.OnProjectileStop`
  (params (ImpactResult :type "HitResult Structure (by ref)"))
  ; Make it cannot damage while stopped
  (set `self.CanDamage` false))

(event `self.CollisionComponent.OnComponentHit`
  (params (HitComponent :type "PrimitiveComponent Object Reference") (OtherActor :type "Actor Object Reference") (OtherComp :type "PrimitiveComponent Object Reference") (NormalImpulse :type "Vector Structure") (Hit :type "HitResult Structure (by ref)"))
  (`KismetSystemLibrary.PrintString` "Arrow Hit!")
  (`GameplayStatics.PlaySoundAtLocation` "/Game/DustinFolder/Audio/SFX/SW_SFX_Arrow_Impact.SW_SFX_Arrow_Impact" (`.Location` (`GameplayStatics.BreakHitResult` Hit)) (struct) 1.0 1.0 0.0 null null null null))

(event `self.ReceiveHit`
  (params (MyComp :type "PrimitiveComponent Object Reference") (Other :type "Actor Object Reference") (OtherComp :type "PrimitiveComponent Object Reference") (bSelfMoved :type Boolean) (HitLocation :type "Vector Structure") (HitNormal :type "Vector Structure") (NormalImpulse :type "Vector Structure") (Hit :type "HitResult Structure (by ref)"))
  ; When Hit the enemy
  (bind _asbp_base_enemy (cast `/Game/RobinProto/Blueprints/Characters/AI/Enemies/BP_BaseEnemy` Other)
    (:`then`
      (if (`self.CanDamage`)
        (bind _findref (`self.GetCharRef` (`self.DamCauserRef`)))
        (`GameplayStatics.ApplyDamage` _asbp_base_enemy (`/Game/RobinProto/Blueprints/Characters/BP_BaseCharacter.Attack` _findref))
        (set `self.CanDamage` false)
        (`self.ResetGravity` :!label _label)))
    (:`CastFailed`
      (goto _label :!via `OtherRoute`))))

(fn `UserConstructionScript`)