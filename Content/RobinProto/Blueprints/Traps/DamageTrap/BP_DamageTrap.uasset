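; BP_DamageTrap is a trap Blueprint that damages and knocks back players that hit it.
; GetHit sets IsColliding and repeats DamagePlayer every tick while that flag is true; nothing in these graphs clears it.
; DamagePlayer checks the player's CanDamageChar, then passes trap damage and knockback forces to DamageCharacter on the BP_SoloGameMode cached at BeginPlay.
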(event `self.ReceiveBeginPlay`
  ; Get Our Gamemode Ref
  (bind _asbp_solo_game_mode (cast `/Game/RobinProto/Blueprints/BP_SoloGameMode` (`GameplayStatics.GetGameMode`)))
  (set `self.GameModeRef` _asbp_solo_game_mode))

(event `/Game/RobinProto/Blueprints/Utilities/BI_Trap.GetHit`
  (params (HitPlayer :type "/Game/RobinProto/Blueprints/Characters/Player/Blueprints/BP_Player Object Reference"))
  ; Damage Player
  (bind _output_get (set `self.IsColliding` true))
  (if _output_get :!label _label
    (`self.DamagePlayer` HitPlayer)
    (`KismetSystemLibrary.DelayUntilNextTick`)
    (goto _label)))

(event `DamagePlayer`
  (params (PlayerRef :type "/Game/RobinProto/Blueprints/Characters/Player/Blueprints/BP_Player Object Reference"))
  ; Damage Player
  (if (`/Game/RobinProto/Blueprints/Characters/BP_BaseCharacter.CanDamageChar` PlayerRef)
    (`/Game/RobinProto/Blueprints/BP_SoloGameMode.DamageCharacter` (`self.GameModeRef`) PlayerRef (`self.TrapDamage`) null null null (`self.KnockbackMainForce`) (`self.KnockbackForceUp`) false)))

(fn `UserConstructionScript`
  (`parent.UserConstructionScript`))