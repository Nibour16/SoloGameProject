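; Game mode for the solo main menu level, which builds the menu UI when play begins.
; BeginPlay switches the first player controller to UI-only input with a visible cursor.
; A CreateWidget helper then adds the main menu to the viewport as visible and the option menu as hidden.
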(event `self.ReceiveBeginPlay`
  ; Initialization
  (`self.SetToUIMode`)
  ;;[1 1 1] Call Main Menu
  (`self.CreateWidget` "/Game/RobinProto/Blueprints/UI/Menus/WBP_MainMenu.WBP_MainMenu_C")
  ;;[1 1 1] Set up Option Menu
  (`self.CreateWidget` "/Game/RobinProto/Blueprints/UI/Menus/WBP_OptionMenu.WBP_OptionMenu_C" "Hidden"))

(event `SetToUIMode`
  (bind _returnvalue (`GameplayStatics.GetPlayerController` 0))
  ; Set UI Mode
  (`WidgetBlueprintLibrary.SetInputMode_UIOnlyEx` _returnvalue null)
  (set `PlayerController.bShowMouseCursor` true _returnvalue))

(fn `CreateWidget`
  (params (NewWidgetClass :type "UserWidget Class Reference") (InVisibility :type "ESlateVisibility Enum" :default "Visible"))
  (bind _returnvalue (`|CreateWidget` NewWidgetClass))
  (`UserWidget.AddToViewport` _returnvalue 0)
  (`Widget.SetVisibility` _returnvalue InVisibility))

(fn `UserConstructionScript`)