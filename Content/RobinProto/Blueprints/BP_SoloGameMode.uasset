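; BP_SoloGameMode is the solo game mode, providing shared helpers for level restart, UI/game mode switching, Enhanced Input setup and character damage.
; SwitchMode toggles cursor, input mode, pause, and visibility of the given widget against the player HUD.
; DamageCharacter applies damage when allowed, then launches the victim using the causer's heading or its own reversed heading, taken from velocity or forward vector.
; Tick binds achievement updates every frame, recording completion in AchivementList.
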(event `self.ReceiveTick`
  (params (DeltaSeconds :type "Float (single-precision)"))
  ; Observe to check when one of the task is complete
  (add `self.OnAchievementUpdated` (delegate `UpdateAchievement`)))

(event `UpdateAchievement` :!signature `self.OnAchievementUpdated`
  (params (AchievementName :type String) (IsTaskCompleted :type Boolean))
  ; Observe to check when one of the task is complete
  (`BlueprintMapLibrary.Map_Add` (`self.AchivementList`) AchievementName IsTaskCompleted))

(fn `DamageCharacter`
  (params (DamagedChar :type "/Game/RobinProto/Blueprints/Characters/BP_BaseCharacter Object Reference") (BaseDamage :type "Float (single-precision)") (EventInstigator :type "Controller Object Reference") (DamageCauser :type "/Game/RobinProto/Blueprints/Characters/BP_BaseCharacter Object Reference") (DamageTypeClass :type "DamageType Class Reference") (MainForce :type "Float (single-precision)") (ExtraForceUp :type "Float (double-precision)") (`Is a Launcher` :type Boolean :default true))
  (locals (SimulatedActor :type "Actor Object Reference"))
  ; Check Can damage char, if can't will return it
  (if (`/Game/RobinProto/Blueprints/Characters/BP_BaseCharacter.CanDamageChar` DamagedChar)
    (`GameplayStatics.ApplyDamage` DamagedChar BaseDamage EventInstigator DamageCauser DamageTypeClass)
    (if (`local.Is a Launcher`)
      ; Launch the damaged Character
      (bind _output_get (set `local.SimulatedActor` (`local.DamageCauser`)))
      (bind _outputforce (`self.LaunchForce` _output_get 1 MainForce ExtraForceUp))
      (`Character.LaunchCharacter` (`local.DamagedChar`) _outputforce false false)
      (else
        (bind _output_get_2 (set `local.SimulatedActor` (`local.DamagedChar`)))
        (bind _outputforce_2 (`self.LaunchForce` _output_get_2 -1 MainForce ExtraForceUp))
        (`Character.LaunchCharacter` (`local.DamagedChar`) _outputforce_2 false false)))
    (else
      (return))))

(fn `MappingContextSetup`
  (params (Controller :type "Object Object Reference") (MappingContext :type "InputMappingContext Object Reference"))
  ; Add Mapping Context
  (bind _asplayer_controller (cast `PlayerController` Controller))
  (bind _returnvalue (pcsubsystem `EnhancedInputLocalPlayerSubsystem` _asplayer_controller))
  (`/Engine/EditorBlueprintResources/StandardMacros.IsValid` _returnvalue
    (:`Is Valid`
      (`EnhancedInputSubsystemInterface.AddMappingContext` _returnvalue MappingContext 1 (struct))
      (bind _returnvalue_2 (`EnhancedInputSubsystemInterface.GetUserSettings` _returnvalue))
      ; Register Mapping Context to Enhanced Input User Setting
      (if (not (`EnhancedInputUserSettings.IsMappingContextRegistered` _returnvalue_2 (`local.MappingContext`)))
        (`EnhancedInputUserSettings.RegisterInputMappingContext` _returnvalue_2 (`local.MappingContext`))))))

(fn `Restart`
  ; Restart By reopening current level
  (bind _returnvalue (`GameplayStatics.GetCurrentLevelName` true))
  (`GameplayStatics.OpenLevel` (`KismetStringLibrary.Conv_StringToName` _returnvalue)))

(fn `SwitchMode`
  (params (`UI ModeWidget` :type "Widget Object Reference (by ref)") (`IsUI Mode` :type Boolean))
  (bind _returnvalue (`GameplayStatics.GetPlayerController` 0))
  (bind _ui_modewidget (`local.UI ModeWidget`))
  ; Switch Mode
  (bind _output_get (set `PlayerController.bShowMouseCursor` `IsUI Mode` _returnvalue))
  (`/Engine/EditorBlueprintResources/StandardMacros.IsValid` `UI ModeWidget`
    (:`Is Valid`
      (if _output_get
        (`WidgetBlueprintLibrary.SetInputMode_GameAndUIEx` _returnvalue `UI ModeWidget` "DoNotLock" false)
        ; Set game paused and show/hide UI Widget
        (`GameplayStatics.SetGamePaused` true)
        (`Widget.SetVisibility` _ui_modewidget "Visible")
        (`self.Hidden/DisplayPlayerHUD` "Hidden")
        (else
          (`WidgetBlueprintLibrary.SetInputMode_GameOnly` _returnvalue :!label _label)
          (`GameplayStatics.SetGamePaused` false)
          (`/Engine/EditorBlueprintResources/StandardMacros.IsValid` _ui_modewidget
            (:`Is Valid`
              (`Widget.SetVisibility` _ui_modewidget "Hidden")
              (`self.Hidden/DisplayPlayerHUD` "Visible"))))))
    (:`Is Not Valid`
      (goto _label))))

(fn `UserConstructionScript`)