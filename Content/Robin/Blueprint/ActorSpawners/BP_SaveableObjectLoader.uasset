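; BP_SaveableObjectLoader restores saved arrows and arrow collectibles from transforms in the game instance's data message.
; LoadObjects triggers LoadArrows, then calls LoadCollectibles with BP_ArrowCollectible.
; Arrows spawn from saved transforms without a save check or cleanup.
; LoadCollectibles acts only when IsSaved is true, destroying every existing actor of the given class before spawning replacements at saved transforms.
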(event `LoadObjects`
  ; Load Objects
  (`self.LoadArrows`)
  (`self.LoadCollectibles` "/Game/RobinProto/Blueprints/Collectibles/BP_ArrowCollectible.BP_ArrowCollectible_C"))

(event `LoadArrows`
  ; Load Objects
  ;;[1 1 1] Load Arrows
  (bind _savedata (message `/Game/Robin/Blueprint/Utilities/BI_SaveGame.GetData` (`GameplayStatics.GetGameInstance`)))
  (`self.Spawn` "/Game/RobinProto/Blueprints/Characters/Projectiles/BP_Arrow.BP_Arrow_C" (`/Game/Robin/Blueprint/DataSave/BP_SaveGame.PlayerArrowTrans` _savedata) "AlwaysSpawn"))

(fn `LoadCollectibles`
  (params (CollectibleClass :type "/Game/RobinProto/Blueprints/Collectibles/BP_BaseCollectible Class Reference"))
  (bind _savedata (message `/Game/Robin/Blueprint/Utilities/BI_SaveGame.GetData` (`GameplayStatics.GetGameInstance`)))
  (if (`/Game/Robin/Blueprint/DataSave/BP_SaveGame.IsSaved` _savedata)
    ; Destroy the collectibles first before spawning
    (bind _outactors (`GameplayStatics.GetAllActorsOfClass` CollectibleClass))
    (for _array_element _outactors
      (`self.K2_DestroyActor` _array_element))
    ; Spawn Actor
    (`self.Spawn` (`local.CollectibleClass`) (`/Game/Robin/Blueprint/DataSave/BP_SaveGame.CollectibleTrans` _savedata) "AlwaysSpawn")
    (return)))

(fn `UserConstructionScript`
  (`parent.UserConstructionScript`))