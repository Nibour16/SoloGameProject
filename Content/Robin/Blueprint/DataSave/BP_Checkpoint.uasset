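; Checkpoint actor that saves player progress to the "Checkpoint" slot when BP_Player overlaps its box.
; One tick after the overlap, it passes the player's data to the game instance for a synchronous save.
; It then stores BP_Arrow transforms in the save data, saves the same slot asynchronously and prints a confirmation.
; Nothing disables the trigger, so each new player overlap saves again.
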(event `self.Box.OnComponentBeginOverlap`
  (params (OverlappedComponent :type "PrimitiveComponent Object Reference") (OtherActor :type "Actor Object Reference") (OtherComp :type "PrimitiveComponent Object Reference") (OtherBodyIndex :type Integer) (bFromSweep :type Boolean) (SweepResult :type "HitResult Structure (by ref)"))
  ; Checkpoint Reached!
  (bind _asbp_player (cast `/Game/RobinProto/Blueprints/Characters/Player/Blueprints/BP_Player` OtherActor))
  (`KismetSystemLibrary.DelayUntilNextTick`)
  (bind _outputdata (`/Game/RobinProto/Blueprints/Characters/Player/Blueprints/BP_Player.GetPlayerData` _asbp_player))
  (message `/Game/Robin/Blueprint/Utilities/BI_SaveGame.SavePlayer` (`GameplayStatics.GetGameInstance`) false _outputdata "Checkpoint")
  (bind _asbp_solo_game_instance (cast `/Game/RobinProto/Blueprints/BP_SoloGameInstance` (`GameplayStatics.GetGameInstance`)))
  (`self.SavePlayerArrows` _asbp_solo_game_instance)
  (`KismetSystemLibrary.PrintString` "GameSaved!"))

(event `SavePlayerArrows`
  (params (GameInstance :type "/Game/RobinProto/Blueprints/BP_SoloGameInstance Object Reference"))
  (bind _outputtransform (message `/Game/Robin/Blueprint/Utilities/BI_SaveGame.SaveTransform` GameInstance "/Game/RobinProto/Blueprints/Characters/Projectiles/BP_Arrow.BP_Arrow_C"))
  (set `/Game/Robin/Blueprint/DataSave/BP_SaveGame.PlayerArrowTrans` _outputtransform (`/Game/RobinProto/Blueprints/BP_SoloGameInstance.SaveGameDataRef` GameInstance))
  (`/Game/RobinProto/Blueprints/BP_SoloGameInstance.SaveData` GameInstance true "Checkpoint"))

(fn `UserConstructionScript`)