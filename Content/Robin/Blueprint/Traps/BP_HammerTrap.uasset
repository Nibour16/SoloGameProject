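; Hammer trap actor that swings continuously back and forth by rotating itself on its roll axis.
; Tick plays or reverses a Timeline according to a direction flag, which flips whenever the animation finishes.
; Timeline alpha interpolates roll between initial and final values, feeding current world pitch and yaw into the actor's relative rotation.
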(event `self.ReceiveTick`
  (params (DeltaSeconds :type "Float (single-precision)"))
  ; Hammer Animation
  (`parent.ReceiveTick` DeltaSeconds)
  (if (`self.IsPositiveRotation`)
    (bind (_direction _alpha) (`Timeline|Timeline` :!label _label)
      (:`Update`
        (`self.UpdateHammer` _alpha))
      (:`Finished`
        (`self.FinishAnimation`)))
    (else
      (goto _label :!via `Reverse`))))

(event `UpdateHammer`
  (params (Alpha :type "Float (double-precision)"))
  (bind (_returnvalue_roll _returnvalue_pitch _returnvalue_yaw) (`KismetMathLibrary.BreakRotator` (`self.K2_GetActorRotation`)))
  ; Update Hammer
  (`self.K2_SetActorRelativeRotation` (`KismetMathLibrary.RLerp` (`KismetMathLibrary.MakeRotator` (`self.InitialRotator`) _returnvalue_pitch _returnvalue_yaw) (`KismetMathLibrary.MakeRotator` (`self.FinalRotator`) _returnvalue_pitch _returnvalue_yaw) Alpha)))

(event `FinishAnimation`
  ; Finish Animation
  (if (`self.IsPositiveRotation`)
    (set `self.IsPositiveRotation` false)
    (else
      (set `self.IsPositiveRotation` true))))

(fn `UserConstructionScript`
  (`parent.UserConstructionScript`))