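; BP_ResetLevelObject is an interactable that resets the level's boxes and arrows when the player uses it.
; On BeginPlay it caches the transform of every BP_Box.
; On Interact by a BP_Player it destroys all BP_Arrow actors, adding one ammo to that player for each.
; It then restores box transforms by array index, relying on GetAllActorsOfClass returning the same order each time.
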(event `self.ReceiveBeginPlay`
  ; Memorize all boxes' initial transform on begin play
  (bind _outactors (`GameplayStatics.GetAllActorsOfClass` "/Game/Robin/Blueprint/BP_Box.BP_Box_C"))
  (for _array_element _outactors
    (`KismetArrayLibrary.Array_Add` (`self.BoxInitialTrans`) (`self.GetTransform` _array_element))))

(event `/Game/RobinProto/Blueprints/Utilities/BlueprintInterfaces/BI_Interactable.Interact`
  (params (Interactor :type "Actor Object Reference"))
  ; On Player Interacted
  (bind _asbp_player (cast `/Game/RobinProto/Blueprints/Characters/Player/Blueprints/BP_Player` Interactor))
  (`self.RestoreArrows` _asbp_player)
  (`self.ResetBoxes`))

(fn `ResetBoxes`
  (bind _outactors (`GameplayStatics.GetAllActorsOfClass` "/Game/Robin/Blueprint/BP_Box.BP_Box_C"))
  (for (_array_element _array_index) _outactors
    (`self.K2_SetActorTransform` _array_element (`|GetArrayItem` (`self.BoxInitialTrans`) _array_index) false false))
  (return))

(fn `RestoreArrows`
  (params (PlayerReference :type "/Game/RobinProto/Blueprints/Characters/Player/Blueprints/BP_Player Object Reference"))
  (bind _outactors (`GameplayStatics.GetAllActorsOfClass` "/Game/RobinProto/Blueprints/Characters/Projectiles/BP_Arrow.BP_Arrow_C"))
  (for _array_element _outactors
    (`self.K2_DestroyActor` _array_element)
    (set `/Game/RobinProto/Blueprints/Characters/Player/Blueprints/BP_Player.CurrentAmmoes` (+ (`/Game/RobinProto/Blueprints/Characters/Player/Blueprints/BP_Player.CurrentAmmoes` PlayerReference) 1) PlayerReference))
  (return))

(fn `UserConstructionScript`)