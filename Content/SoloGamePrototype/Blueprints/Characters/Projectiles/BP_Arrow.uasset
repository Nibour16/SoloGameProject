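; BP_Arrow is an arrow projectile that damages enemies and can be picked up by the player to restore ammo.
; On hit, it damages any BP_BaseEnemy, then turns on bounce and normal gravity in the ResetGravity graph.
; Any other hit turns off bounce and gravity instead.
; Interacting as BP_Player calls CollectArrow to return one arrow, then destroys the actor.
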(event `/Game/SoloGamePrototype/Blueprints/Utilities/BI_Interactable.Interact`
  (params (Interactor :type "Actor Object Reference"))
  ; Interact this actor to restore the arrow
  (bind _asbp_player (cast `/Game/SoloGamePrototype/Blueprints/Characters/Player/Blueprints/BP_Player` Interactor))
  (`/Game/SoloGamePrototype/Blueprints/Characters/Player/Blueprints/BP_Player.CollectArrow` _asbp_player 1)
  (`self.K2_DestroyActor`))

(event `self.ReceiveHit`
  (params (MyComp :type "PrimitiveComponent Object Reference") (Other :type "Actor Object Reference") (OtherComp :type "PrimitiveComponent Object Reference") (bSelfMoved :type Boolean) (HitLocation :type "Vector Structure") (HitNormal :type "Vector Structure") (NormalImpulse :type "Vector Structure") (Hit :type "HitResult Structure (by ref)"))
  ; When Hit the enemy
  (bind _asbp_base_enemy (cast `/Game/SoloGamePrototype/Blueprints/Characters/AI/BP_BaseEnemy` Other)
    (:`then`
      (`self.DamageActor` _asbp_base_enemy)
      (`self.ResetGravity` :!label _label))
    (:`CastFailed`
      (goto _label :!via `OtherRoute`))))

(fn `UserConstructionScript`)