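; Base character Blueprint that provides health, damage handling and a temporary invincibility window.
; Health starts at MaxHealth on BeginPlay, and AnyDamage feeds GetDamaged, which subtracts the damage and then checks the result.
; Zero or lower health calls WhenDied, otherwise the remaining health is printed.
; A separate PlayerInvincible event disables CanBeDamaged, waits for the passed character's InvicibleTime, then re-enables it.
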(event `self.ReceiveBeginPlay`
  ; Initialize Health
  (set `self.CurrentHealth` (`self.MaxHealth`)))

(event `self.ReceiveAnyDamage`
  (params (Damage :type "Float (single-precision)") (DamageType :type "DamageType Object Reference") (InstigatedBy :type "Controller Object Reference") (DamageCauser :type "Actor Object Reference"))
  ; Get Damaged
  (`self.GetDamaged` Damage))

(event `PlayerInvincible`
  (params (CharRef :type "/Game/SoloGamePrototype/Blueprints/Characters/BP_BaseCharacter Object Reference"))
  ; Invincible a while after they get hit
  (set `self.CanBeDamaged` false)
  (`KismetSystemLibrary.Delay` (`/Game/SoloGamePrototype/Blueprints/Characters/Player/Blueprints/BP_Player.InvicibleTime` CharRef))
  (set `self.CanBeDamaged` true))

(fn `CalcDamage`
  (params (Damage :type "Float (double-precision)"))
  (set `self.CurrentHealth` (- (`self.CurrentHealth`) Damage))
  (return))

(fn `DamageResult`
  (if (<= (`self.CurrentHealth`) 0.0)
    (`self.WhenDied`)
    (else
      (`KismetSystemLibrary.PrintString` (`KismetStringLibrary.Conv_DoubleToString` (`self.CurrentHealth`))))))

(fn `GetDamaged`
  (params (Damage :type "Float (double-precision)"))
  (`self.CalcDamage` Damage)
  (`self.DamageResult`))

(fn `UserConstructionScript`)