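; BP_OutOfBound is a level boundary volume that handles anything overlapping its LevelBoundary component.
; An overlapping player triggers Restart on BP_SoloGameMode.
; An overlapping player arrow is destroyed, first returning one arrow to the player if CanReturnPlayerProjectilesFromBoundary is set.
; Any other overlapping actor is simply destroyed.
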(event `self.LevelBoundary.OnComponentBeginOverlap`
  (params (OverlappedComponent :type "PrimitiveComponent Object Reference") (OtherActor :type "Actor Object Reference") (OtherComp :type "PrimitiveComponent Object Reference") (OtherBodyIndex :type Integer) (bFromSweep :type Boolean) (SweepResult :type "HitResult Structure (by ref)"))
  ; When Something Overlaps
  (cast `/Game/SoloGamePrototype/Blueprints/Characters/Player/Blueprints/BP_Player` OtherActor
    (:`then`
      (`self.PlayerOutOfBound!`))
    (:`CastFailed`
      (bind _asbp_arrow (cast `/Game/SoloGamePrototype/Blueprints/Characters/Projectiles/BP_Arrow` OtherActor)
        (:`then`
          (`self.PlayerProjectileOutOfBound!` _asbp_arrow))
        (:`CastFailed`
          (`self.K2_DestroyActor` OtherActor) ; Destroy Actor if other actor is out of bound
        )))))

(event `PlayerOutOfBound!`
  ; Out of Bound!
  (bind _asbp_solo_game_mode (cast `/Game/SoloGamePrototype/Blueprints/BP_SoloGameMode` (`GameplayStatics.GetGameMode`)))
  (`/Game/SoloGamePrototype/Blueprints/BP_SoloGameMode.Restart` _asbp_solo_game_mode))

(event `PlayerProjectileOutOfBound!`
  (params (PlayerProjectile :type "Actor Object Reference"))
  ; Return Player's Arrow if their arrow is out of bound
  (bind _asbp_player (cast `/Game/SoloGamePrototype/Blueprints/Characters/Player/Blueprints/BP_Player` (`GameplayStatics.GetPlayerCharacter` 0)))
  (if (`/Game/SoloGamePrototype/Blueprints/Characters/Player/Blueprints/BP_Player.CanReturnPlayerProjectilesFromBoundary` _asbp_player)
    (`/Game/SoloGamePrototype/Blueprints/Characters/Player/Blueprints/BP_Player.CollectArrow` _asbp_player 1))
  (`self.K2_DestroyActor` PlayerProjectile))

(fn `UserConstructionScript`)