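; BP_BreakableWall is a wall actor that loses one health point per hit and is destroyed when its health reaches zero.
; The OnWallGetHit event decrements WallHealth, updates two text renders showing the remaining health, and swaps the wall mesh to BrokenMaterial when health equals BrokenHealth.
; The construction script sets both displays to the starting health and applies TextColor, so the values preview in the editor.
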(event `/Game/Robin/Blueprint/Utilities/BI_SpecialWallInteraction.OnWallGetHit`
  (bind _result (`/Engine/EditorBlueprintResources/StandardMacros.DecrementInt` (`self.WallHealth`))
    (:`  `
      (bind _output_get (set `self.WallHealth` _result))
      (`TextRenderComponent.K2_SetText` (`self.WallHealthDisplay`) (`KismetTextLibrary.Conv_IntToText` _output_get))
      (`TextRenderComponent.K2_SetText` (`self.WallHealthDisplay1`) (`KismetTextLibrary.Conv_IntToText` _output_get))
      (if (<= _output_get 0)
        (`self.K2_DestroyActor`)
        (elif (== _output_get (`self.BrokenHealth`))
          (`PrimitiveComponent.SetMaterial` (`self.WallMesh`) 0 (`self.BrokenMaterial`)))))))

(fn `UserConstructionScript`
  (`TextRenderComponent.K2_SetText` (`self.WallHealthDisplay`) (`KismetTextLibrary.Conv_IntToText` (`self.WallHealth`)))
  (`TextRenderComponent.K2_SetText` (`self.WallHealthDisplay1`) (`KismetTextLibrary.Conv_IntToText` (`self.WallHealth`)))
  (`TextRenderComponent.SetTextRenderColor` (`self.WallHealthDisplay`) (`self.TextColor`))
  (`TextRenderComponent.SetTextRenderColor` (`self.WallHealthDisplay1`) (`self.TextColor`)))