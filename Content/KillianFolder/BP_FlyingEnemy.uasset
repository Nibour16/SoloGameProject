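; BP_FlyingEnemy is a flying enemy Blueprint that can fire projectiles.
; Its ShootProjectile event prints a debug string and spawns ProjectileClass at the ShootingPos component, offset by ProjectileOffset and using that component's rotation.
; The construction script applies EnemyTransform as the relative transform of both Sphere and AttackBox, then runs the parent construction script.
; Nothing in this graph calls ShootProjectile, and an unconnected raycast check remains.
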(event `ShootProjectile`
  (bind _shootingpos (`self.ShootingPos`))
  ; Shoot a projectile
  (`KismetSystemLibrary.PrintString` "Shoot!")
  (`|SpawnActorFromClass` (`self.Projectile Class`) (`KismetMathLibrary.MakeTransform` (+ (`SceneComponent.K2_GetComponentLocation` _shootingpos) (`self.Projectile Offset`)) (`SceneComponent.K2_GetComponentRotation` _shootingpos)) "Undefined" "MultiplyWithRoot" null null))

(fn `UserConstructionScript`
  (`SceneComponent.K2_SetRelativeTransform` (`self.Sphere`) (`self.EnemyTransform`) false false)
  (`SceneComponent.K2_SetRelativeTransform` (`self.AttackBox`) (`self.EnemyTransform`) false false)
  (`parent.UserConstructionScript`))